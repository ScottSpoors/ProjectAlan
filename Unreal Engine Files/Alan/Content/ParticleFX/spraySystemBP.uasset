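; Spray-paint effect Blueprint that fires a particle system and plays a spray sound when the player presses Space.
; On BeginPlay it enables input from player controller 0 so it can read keys directly.
; Number keys 0 to 7 recolour the spray by setting the particle system's "Colour" parameter to preset colours.
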(event EventBeginPlay
  (Input|EnableInput (Game|GetPlayerController 0)))

(event Input|KeyboardEvents|SpaceBar
  (params (Key :type Key%20Structure :default "None"))
  (:Pressed
    (Components|Activation|Activate (Variables|Default|GetspraySystem) false)
    (Audio|PlaySound2D "/Game/Audio/Spraysounds/spraySounds.spraySounds" 1.0 1.0 0.0 0 0)))

(event Input|KeyboardEvents|0
  (params (Key :type Key%20Structure :default "None"))
  (:Pressed
    (Effects|Components|ParticleSystem|SetColorParameter (Variables|Default|GetspraySystem) "Colour" (Class|KismetMathLibrary|LinearColorBlack))))

(event Input|KeyboardEvents|1
  (params (Key :type Key%20Structure :default "None"))
  (:Pressed
    (Effects|Components|ParticleSystem|SetColorParameter (Variables|Default|GetspraySystem) "Colour" (Class|KismetMathLibrary|LinearColorWhite))))

(event Input|KeyboardEvents|2
  (params (Key :type Key%20Structure :default "None"))
  (:Pressed
    (Effects|Components|ParticleSystem|SetColorParameter (Variables|Default|GetspraySystem) "Colour" (Utilities|Struct|MakeLinearColor 255.0 192.0 203.0 0.1))))

(event Input|KeyboardEvents|3
  (params (Key :type Key%20Structure :default "None"))
  (:Pressed
    (Effects|Components|ParticleSystem|SetColorParameter (Variables|Default|GetspraySystem) "Colour" (Class|KismetMathLibrary|LinearColorBlue))))

(event Input|KeyboardEvents|6
  (params (Key :type Key%20Structure :default "None"))
  (:Pressed
    (Effects|Components|ParticleSystem|SetColorParameter (Variables|Default|GetspraySystem) "Colour" (Class|KismetMathLibrary|LinearColorYellow))))

(event Input|KeyboardEvents|4
  (params (Key :type Key%20Structure :default "None"))
  (:Pressed
    (Effects|Components|ParticleSystem|SetColorParameter (Variables|Default|GetspraySystem) "Colour" (Utilities|Struct|MakeLinearColor 159.0 43.0 104.0 0.1))))

(event Input|KeyboardEvents|5
  (params (Key :type Key%20Structure :default "None"))
  (:Pressed
    (Effects|Components|ParticleSystem|SetColorParameter (Variables|Default|GetspraySystem) "Colour" (Class|KismetMathLibrary|LinearColorGreen))))

(event Input|KeyboardEvents|7
  (params (Key :type Key%20Structure :default "None"))
  (:Pressed
    (Effects|Components|ParticleSystem|SetColorParameter (Variables|Default|GetspraySystem) "Colour" (Utilities|Struct|MakeLinearColor 255.0 165.0 0.0 0.1))))

(fn ConstructionScript)